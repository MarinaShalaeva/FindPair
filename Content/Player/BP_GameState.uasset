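; BP_GameState is a game state Blueprint that creates and wires up the card system objects when play begins.
; It constructs a shared CPP_CardsDelegates object and a CPP_SpawnCardsManager, which it initializes with that delegates reference.
; It then loops until player controller 0 is valid, casts it to CPP_PlayerController and passes it the same delegates object.
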(event EventBeginPlay
  (Utilities|FlowControl|Sequence
    (:then_0
      (bind _returnvalue (Game|ConstructObjectfromClass self "/Script/FindPair.CPP_CardsDelegates"))
      (Variables|Default|SetCardsDelegatesRef _returnvalue))
    (:then_1
      (bind _returnvalue_2 (Game|ConstructObjectfromClass self "/Script/FindPair.CPP_SpawnCardsManager"))
      (bind _output_get (Variables|Default|SetSpawnCardsManager _returnvalue_2))
      (Class|CPPSpawnCardsManager|InitializeCardsDelegatesVariable _output_get (Variables|Default|GetCardsDelegatesRef)))
    (:then_2
      (while (not (Utilities|IsValid (Game|GetPlayerController 0)))
        _)
      (bind _ascpp_player_controller (Utilities|Casting|CastToCPP_PlayerController (Game|GetPlayerController 0)))
      (Class|CPPPlayerController|SetCardsDelegatesRef _ascpp_player_controller (Variables|Default|GetCardsDelegatesRef)))))

(fn ConstructionScript)